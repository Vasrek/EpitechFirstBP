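; BP_Platform is a platform actor that reacts to the player stepping on it according to its PlatformType.
; A box trigger detects the player character, and for the Falling Platform type the cube begins simulating physics after a short delay.
; Several seconds later, physics is switched off and the cube teleports back to the transform cached at BeginPlay.
; The FakePlatform event is an empty stub.
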(event `self.ReceiveBeginPlay`
  (set `self.DefaultTransform` (`SceneComponent.K2_GetComponentToWorld` (`self.Cube`))))

(event `self.Box.OnComponentBeginOverlap`
  (params (OverlappedComponent :type "PrimitiveComponent Object Reference") (OtherActor :type "Actor Object Reference") (OtherComp :type "PrimitiveComponent Object Reference") (OtherBodyIndex :type Integer) (bFromSweep :type Boolean) (SweepResult :type "HitResult Structure (by ref)"))
  (if (== OtherActor (`GameplayStatics.GetPlayerCharacter` 0))
    (switch `/Game/Blueprints/Actors/E_PlatformTypes` (`self.PlatformType`)
      (:`NewEnumerator0`
        (`self.FallingPlatform`)))))

(event `FallingPlatform`
  (`KismetSystemLibrary.Delay` 1.0)
  (`PrimitiveComponent.SetSimulatePhysics` (`self.Cube`) true)
  (`KismetSystemLibrary.Delay` 5.0)
  (`PrimitiveComponent.SetSimulatePhysics` (`self.Cube`) false)
  (`SceneComponent.K2_SetWorldTransform` (`self.Cube`) (`self.DefaultTransform`) false true))

(event `FakePlatform`)

(fn `UserConstructionScript`)