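; BP_FakePlatform is a paired-platform trap that randomly makes one of its two platforms fake.
; BeginPlay picks the fake side and calls ChangePlatformColor on the right platform regardless of the result.
; Player overlap with either trigger box runs the same logic, so the fake platform drops whichever box is entered.
; The drop enables physics simulation on that component, then destroys it after a short delay.
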(event `self.ReceiveBeginPlay`
  (`parent.ReceiveBeginPlay`)
  (if (== (`KismetMathLibrary.RandomIntegerInRange` 0 1) 0)
    (set `self.IsLeftFake?` true)
    (else
      (set `self.IsLeftFake?` false)))
  (`self.ChangePlatformColor` (`self.RightPlatform`)))

(event `self.RightBoxCol.OnComponentBeginOverlap`
  (params (OverlappedComponent :type "PrimitiveComponent Object Reference") (OtherActor :type "Actor Object Reference") (OtherComp :type "PrimitiveComponent Object Reference") (OtherBodyIndex :type Integer) (bFromSweep :type Boolean) (SweepResult :type "HitResult Structure (by ref)"))
  (bind _platformtodestroy (`self.PlatformToDestroy`))
  (if (== OtherActor (`GameplayStatics.GetPlayerCharacter` 0))
    (if (`self.IsLeftFake?`) :!label _label
      (set `self.PlatformToDestroy` (`self.Cube`))
      (else
        (set `self.PlatformToDestroy` (`self.RightPlatform`))))
    (`/Engine/EditorBlueprintResources/StandardMacros.IsValid` (`self.PlatformToDestroy`)
      (:`Is Valid`
        (`PrimitiveComponent.SetSimulatePhysics` _platformtodestroy true)
        (`KismetSystemLibrary.Delay` 5.0)
        (`ActorComponent.K2_DestroyComponent` _platformtodestroy)))))

(event `self.Box.OnComponentBeginOverlap`
  (params (OverlappedComponent :type "PrimitiveComponent Object Reference") (OtherActor :type "Actor Object Reference") (OtherComp :type "PrimitiveComponent Object Reference") (OtherBodyIndex :type Integer) (bFromSweep :type Boolean) (SweepResult :type "HitResult Structure (by ref)"))
  (if (== OtherActor (`GameplayStatics.GetPlayerCharacter` 0))
    (goto _label)))

(fn `UserConstructionScript`
  (`parent.UserConstructionScript`))