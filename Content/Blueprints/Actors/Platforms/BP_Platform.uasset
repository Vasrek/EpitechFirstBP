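; BP_Platform is a platform actor whose behavior depends on a PlatformType enum, with only the falling type implemented.
; On BeginPlay it saves the cube's transform and assigns one of six random color materials.
; When the player character overlaps the box, a falling platform waits briefly, enables physics on the cube, then later stops simulation and teleports it back to its saved transform.
; The FakePlatform event is an empty stub.
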(event `self.ReceiveBeginPlay`
  ;[0 1 0.03793] Save default transform
  (set `self.DefaultTransform` (`SceneComponent.K2_GetComponentToWorld` (`self.Cube`)))
  (`self.ChangePlatformColor` (`self.Cube`)))

(event `self.Box.OnComponentBeginOverlap`
  (params (OverlappedComponent :type "PrimitiveComponent Object Reference") (OtherActor :type "Actor Object Reference") (OtherComp :type "PrimitiveComponent Object Reference") (OtherBodyIndex :type Integer) (bFromSweep :type Boolean) (SweepResult :type "HitResult Structure (by ref)"))
  ;[0 1 0.03793] On overlap check which type of platform and call the correct event
  (if (== OtherActor (`GameplayStatics.GetPlayerCharacter` 0))
    (switch `/Game/Blueprints/Actors/Platforms/E_PlatformTypes` (`self.PlatformType`)
      (:`NewEnumerator0`
        (`self.FallingPlatform`)))))

(event `FallingPlatform`
  ;[0 1 0.03793] Falling platform after 1 sec - respawn it after 5 seconds
  (`KismetSystemLibrary.Delay` 1.0)
  (`PrimitiveComponent.SetSimulatePhysics` (`self.Cube`) true)
  (`KismetSystemLibrary.Delay` 5.0)
  (`PrimitiveComponent.SetSimulatePhysics` (`self.Cube`) false)
  (`SceneComponent.K2_SetWorldTransform` (`self.Cube`) (`self.DefaultTransform`) false true))

(event `FakePlatform`)

(fn `ChangePlatformColor`
  (params (CubeToChangeColor :type "StaticMeshComponent Object Reference"))
  (switch `int` (`KismetMathLibrary.RandomIntegerInRange` 0 5)
    (:`0`
      (set `self.MaterialToSet` "/Game/Materials/M_Blue.M_Blue"))
    (:`1`
      (set `self.MaterialToSet` "/Game/Materials/M_Brown.M_Brown"))
    (:`2`
      (set `self.MaterialToSet` "/Game/Materials/M_Green.M_Green"))
    (:`3`
      (set `self.MaterialToSet` "/Game/Materials/M_Orange.M_Orange"))
    (:`4`
      (set `self.MaterialToSet` "/Game/Materials/M_Red.M_Red"))
    (:`5`
      (set `self.MaterialToSet` "/Game/Materials/M_Yellow.M_Yellow")))
  (`PrimitiveComponent.SetMaterial` CubeToChangeColor 0 (`self.MaterialToSet`)))

(fn `UserConstructionScript`)