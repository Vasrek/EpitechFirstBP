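; Player character for a game with score, checkpoints and respawning, driven by camera-relative movement, mouse look and jump.
; BeginPlay saves the starting transform as the respawn point and creates the HUD widget, which receives every score change.
; Respawn teleports to the saved transform and deducts a death penalty while score is positive; setting a new checkpoint plays a placeholder sound.
; The win event only prints a message so far.
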(event `InputAxis|MoveForward/BackWard`
  (params (AxisValue :type "Float (single-precision)"))
  (bind (_returnvalue_roll _returnvalue_pitch _returnvalue_yaw) (`KismetMathLibrary.BreakRotator` (`self.GetControlRotation`)))
  ;[1 0.9217 0] Input : Movement / Camera (mouse)
  (`self.AddMovementInput` (`KismetMathLibrary.GetForwardVector` (`KismetMathLibrary.MakeRotator` 0.0 0.0 _returnvalue_yaw)) AxisValue))

(event `InputAction|Jump`
  (params (Key :type "Key Structure"))
  ;[1 0.9217 0] Input : Movement / Camera (mouse)
  (:`Pressed`
    (`self.Jump`))
  (:`Released`
    (`self.StopJumping`)))

(event `IncreaseScore`
  (params (ScoreToAdd :type Integer))
  ;[0 0 0 1 35] Main features
  ;;[0 1 0.03793] Add score + display the score
  (bind _output_get (set `self.TotalScore` (+ ScoreToAdd (`self.TotalScore`))))
  (`/Game/Blueprints/Widgets/WBP_Hud.UpdateScore` (`self.HUD_Ref`) _output_get))

(event `Respawn`
  ;[0 0 0 1 35] Main features
  ;;[0 1 0.03793] Respawn to last Player Respawn Transform
  (`self.K2_SetActorTransform` (`self.PlayerRespawnTransform`) false true)
  (`self.ReduceScore` (`self.DeathAmountScore`)))

(event `InputAxis|MouseLook`
  (params (AxisValue :type "Float (single-precision)"))
  ;[1 0.9217 0] Input : Movement / Camera (mouse)
  (`self.AddControllerYawInput` AxisValue))

(event `InputAxis|MoveRight/Left`
  (params (AxisValue :type "Float (single-precision)"))
  (bind (_returnvalue_roll _returnvalue_pitch _returnvalue_yaw) (`KismetMathLibrary.BreakRotator` (`self.GetControlRotation`)))
  ;[1 0.9217 0] Input : Movement / Camera (mouse)
  (`self.AddMovementInput` (`KismetMathLibrary.GetRightVector` (`KismetMathLibrary.MakeRotator` 0.0 0.0 _returnvalue_yaw)) AxisValue))

(event `InputAxis|MouseLookUp`
  (params (AxisValue :type "Float (single-precision)"))
  ;[1 0.9217 0] Input : Movement / Camera (mouse)
  (`self.AddControllerPitchInput` AxisValue))

(event `ReduceScore`
  (params (ScoreToSubstract :type Integer))
  ;[0 0 0 1 35] Main features
  ;;[0 1 0.03793] Substract X and set it to Total score + Update score to HUD
  (if (not (<= (`self.TotalScore`) 0))
    (bind _output_get (set `self.TotalScore` (- (`self.TotalScore`) ScoreToSubstract)))
    (`/Game/Blueprints/Widgets/WBP_Hud.UpdateScore` (`self.HUD_Ref`) _output_get)))

(event `self.ReceiveBeginPlay`
  ;[0 0 0 1 35] Main features
  ;;[0 1 0.03793] BeginPlay: SaveCurrent transform to PlayerRespawnTransform + create hud
  (set `self.PlayerRespawnTransform` (`self.GetTransform`))
  (bind _returnvalue (`|CreateWidget` "/Game/Blueprints/Widgets/WBP_Hud.WBP_Hud_C"))
  (bind _output_get (set `self.HUD_Ref` _returnvalue))
  (`UserWidget.AddToViewport` _output_get 0))

(event `PlayerWon`
  ;[0 0 0 1 35] Main features
  ;;[1 0.06771 0.06771] TODO Win condition
  (`KismetSystemLibrary.PrintString` "The player has finish the game!"))

(event `SetNewRespawnTransform`
  (params (NewPlayerRespawnTransform :type "Transform Structure"))
  ;[0 0 0 1 35] Main features
  ;;[0 1 0.03793] Set new respawn transform
  (set `self.PlayerRespawnTransform` NewPlayerRespawnTransform)
  ;;;[1 0.06771 0.06771] TODO Change checkpoint SFX
  (`GameplayStatics.PlaySound2D` "/Game/StarterContent/Audio/Explosion01.Explosion01" 1.0 1.0 0.0 null null))

(fn `UserConstructionScript`)